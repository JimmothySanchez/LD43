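; BP_Liam is a character Blueprint that handles camera-relative movement input.
; The forward and right axis events feed scaled direction vectors straight into CharacterMovement as input.
; Directions come from a look-at rotation from player camera 0's location to the actor, so movement follows the camera's viewpoint rather than control rotation.
; SetControlRotation calls and axis-rotation nodes remain in the graph but never run.
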(event EventBeginPlay)

(event Collision|EventActorBeginOverlap
  (params (OtherActor :type Actor%20Object%20Reference)))

(event EventTick
  (params (DeltaSeconds :type Float%20%28single-precision%29)))

(event Input|AxisEvents|InputAxisInput_Forward
  (params (AxisValue :type Float%20%28single-precision%29))
  (Class|PawnMovementComponent|AddInputVector (Variables|Character|GetCharacterMovement) (* (Math|Vector|GetForwardVector (Math|Rotator|FindLookatRotation (Camera|GetCameraLocation (Game|GetPlayerCameraManager 0)) (Transformation|GetActorLocation))) AxisValue) false))

(event Input|AxisEvents|InputAxisInput_Right
  (params (AxisValue :type Float%20%28single-precision%29))
  (Class|PawnMovementComponent|AddInputVector (Variables|Character|GetCharacterMovement) (* (Math|Vector|GetRightVector (Math|Rotator|FindLookatRotation (Camera|GetCameraLocation (Game|GetPlayerCameraManager 0)) (Transformation|GetActorLocation))) AxisValue) false))

(fn ConstructionScript)