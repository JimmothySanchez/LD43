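; Player character Liam, built from separate body parts that break apart when he dies from a long fall.
; Axis input moves him relative to the camera-to-character direction and sets control rotation to face the input.
; Tick tracks fall start height; landing beyond MaxFallDistance fires LiamDied and detaches head, hands and feet as physics bodies.
; UpdateAnim is an empty stub, and FallStraightDown, which swaps the body for a BP_TorsoBlock, is only called from disconnected logic.
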(event EventBeginPlay)

(event Collision|EventActorBeginOverlap
  (params (OtherActor :type Actor%20Object%20Reference)))

(event EventTick
  (params (DeltaSeconds :type Float%20%28single-precision%29))
  (CallFunction|UpdateFalling))

(event Input|AxisEvents|InputAxisInput_Forward
  (params (AxisValue :type Float%20%28single-precision%29))
  (bind _returnvalue (Game|GetPlayerCameraManager 0))
  (bind _returnvalue_2 (Transformation|GetActorLocation))
  (bind _returnvalue_3 (Camera|GetCameraLocation _returnvalue))
  (bind _returnvalue_4 (Math|Rotator|FindLookatRotation _returnvalue_3 _returnvalue_2))
  (bind _returnvalue_5 (Math|Vector|GetForwardVector _returnvalue_4))
  (bind _returnvalue_6 (* _returnvalue_5 AxisValue))
  (Class|PawnMovementComponent|AddInputVector (Variables|Character|GetCharacterMovement) _returnvalue_6 false)
  (CallFunction|UpdateRot _returnvalue_6)
  (CallFunction|UpdateAnim "0, 0, 0"))

(event Input|AxisEvents|InputAxisInput_Right
  (params (AxisValue :type Float%20%28single-precision%29))
  (bind _returnvalue (Game|GetPlayerCameraManager 0))
  (bind _returnvalue_2 (Transformation|GetActorLocation))
  (bind _returnvalue_3 (Camera|GetCameraLocation _returnvalue))
  (bind _returnvalue_4 (Math|Rotator|FindLookatRotation _returnvalue_3 _returnvalue_2))
  (bind _returnvalue_5 (Math|Vector|GetRightVector _returnvalue_4))
  (bind _returnvalue_6 (* _returnvalue_5 AxisValue))
  (Class|PawnMovementComponent|AddInputVector (Variables|Character|GetCharacterMovement) _returnvalue_6 false)
  (CallFunction|UpdateRot _returnvalue_6)
  (CallFunction|UpdateAnim "0, 0, 0"))

(fn ConstructionScript)

(fn UpdateRot
  (params (IncomingDirection :type Vector))
  (if (> (Math|Vector|VectorLength IncomingDirection) 0.0)
    (Pawn|SetControlRotation (Pawn|GetController) (Math|Rotator|MakeRotationfromAxes IncomingDirection "0, 0, 0" "0, 0, 0"))))

(fn UpdateFalling
  (if (Math|Boolean|NotEqual(Boolean) (AI|Components|NavMovement|IsFalling (Variables|Character|GetCharacterMovement)) (Variables|Falling|GetFalling))
    (if (and (AI|Components|NavMovement|IsFalling (Variables|Character|GetCharacterMovement)) (not (Variables|Default|GetDead)))
      (Variables|Falling|SetInitialFallHeight (.Z (Math|Vector|BreakVector (Transformation|GetActorLocation self))))
      (Variables|Falling|SetFalling true)
      (elif (>= (Math|Float|Absolute(Float) (- (Variables|Falling|GetInitialFallHeight) (.Z (Math|Vector|BreakVector (Transformation|GetActorLocation self))))) (Variables|Default|GetMaxFallDistance))
        (CallFunction|Die)
        (else
          (Variables|Falling|SetFalling false))))))

(fn Die
  (Default|CallLiamDied)
  (Utilities|FlowControl|Sequence
    (:then_0
      (Transformation|DetachFromComponent (Variables|Default|GetHead) "KeepWorld" "KeepWorld" "KeepWorld" true)
      (Physics|SetSimulatePhysics (Variables|Default|GetHead) true))
    (:then_1
      (Transformation|DetachFromComponent (Variables|Default|GetHand_L) "KeepWorld" "KeepWorld" "KeepWorld" true)
      (Physics|SetSimulatePhysics (Variables|Default|GetHand_L) true))
    (:then_2
      (Transformation|DetachFromComponent (Variables|Default|GetHand_R) "KeepWorld" "KeepWorld" "KeepWorld" true)
      (Physics|SetSimulatePhysics (Variables|Default|GetHand_R) true))
    (:then_3
      (Transformation|DetachFromComponent (Variables|Default|GetFoot_R) "KeepWorld" "KeepWorld" "KeepWorld" true)
      (Physics|SetSimulatePhysics (Variables|Default|GetFoot_R) true))
    (:then_4
      (Transformation|DetachFromComponent (Variables|Default|GetFoot_L) "KeepWorld" "KeepWorld" "KeepWorld" true)
      (Physics|SetSimulatePhysics (Variables|Default|GetFoot_L) true))))

(fn UpdateAnim
  (params (Direction :type Vector))
  (if (and (> (Math|Vector|VectorLength Direction) 0.0) (not (Variables|Default|GetDead)))
    _))

(fn FallStraightDown
  (bind _liam (Variables|Default|GetLiam))
  (LocalVariables|SetlclBodyTransform (Transformation|GetWorldTransform _liam))
  (Components|DestroyComponent _liam)
  (Game|SpawnActorfromClass "/Game/CustomLD43/Actors/Character/BP_TorsoBlock.BP_TorsoBlock_C" (LocalVariables|GetlclBodyTransform) "Undefined" 0 true 0)
  (Variables|Default|SetDead true))