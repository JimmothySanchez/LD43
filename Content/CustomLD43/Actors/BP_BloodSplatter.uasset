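; BP_BloodSplatter is a blood decal actor that spreads and changes opacity to look like bleeding out.
; On BeginPlay it creates a dynamic instance of Mat_Blood_Decal_Inst and assigns it to its Decal component.
; Each Tick, until the actor's age reaches BleedOutTime, it lerps the material's OpacityMultiplier and the decal's uniform world scale between their min and max values.
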(event EventBeginPlay
  (bind _returnvalue (Rendering|Material|CreateDynamicMaterialInstance (Variables|/Script/Engine.DecalComponent|GetDecalMaterial (Variables|Default|GetDecal)) "/Game/CustomLD43/RawAssets/Blood/Mat_Blood_Decal_Inst.Mat_Blood_Decal_Inst" "None" :!class /Script/Engine.KismetMaterialLibrary))
  (bind _output_get (Variables|Default|SetMatInstance _returnvalue))
  (Rendering|Components|Decal|SetDecalMaterial (Variables|Default|GetDecal) _output_get))

(event Collision|EventActorBeginOverlap
  (params (OtherActor :type Actor%20Object%20Reference)))

(event EventTick
  (params (DeltaSeconds :type Float%20%28single-precision%29))
  (bind _returnvalue (Actor|GetGameTimeSinceCreation))
  (bind _maxscale (Variables|Default|GetMaxSCale))
  (bind _minscale (Variables|Default|GetMinScale))
  (bind _bleedouttime (Variables|Default|GetBleedOutTime))
  (bind _returnvalue_2 (/ _returnvalue _bleedouttime))
  (bind _returnvalue_3 (Math|Float|Lerp _minscale _maxscale _returnvalue_2))
  (if (< (Actor|GetGameTimeSinceCreation) (Variables|Default|GetBleedOutTime))
    (Utilities|FlowControl|Sequence
      (:then_0
        (Rendering|Material|SetScalarParameterValue (Variables|Default|GetMatInstance) "OpacityMultiplier" (Math|Float|Lerp (Variables|Default|GetMinOpacity) (Variables|Default|GetMaxOpacity) (/ (Actor|GetGameTimeSinceCreation) (Variables|Default|GetBleedOutTime))) :!class /Script/Engine.MaterialInstanceDynamic))
      (:then_1
        (Transformation|SetWorldScale3D (Variables|Default|GetDecal) (Math|Vector|MakeVector _returnvalue_3 _returnvalue_3 _returnvalue_3))))))

(fn ConstructionScript)