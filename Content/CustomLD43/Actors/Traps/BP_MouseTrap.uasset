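; BP_MouseTrap is a trap actor that snaps shut and kills the player.
; When the player pawn overlaps its Box, a DoOnce sets the triggered flag, calls Triggered, calls Die on BP_Liam_Parts and plays the snap sound.
; Tick then swings the Clamp closed by lerping its relative rotation over SnapDuration.
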(event OnComponentBeginOverlap(Box)
  (params (OverlappedComponent :type Primitive%20Component%20Object%20Reference) (OtherActor :type Actor%20Object%20Reference) (OtherComp :type Primitive%20Component%20Object%20Reference) (OtherBodyIndex :type Integer) (bFromSweep :type Boolean) (SweepResult :type Hit%20Result%20Structure%20%28by%20ref%29))
  (if (== OtherActor (Game|Player|GetPlayerPawn 0))
    (Utilities|FlowControl|DoOnce false
      (:Completed
        (Utilities|FlowControl|Sequence
          (:then_0
            (Variables|Default|SetboolTriggered true)
            (Default|CallTriggered))
          (:then_1
            (bind _asbp_liam_parts (Utilities|Casting|CastToBP_Liam_Parts OtherActor))
            (Default|Die _asbp_liam_parts)
            (Audio|PlaySound2D "/Game/CustomLD43/Audio/FX/Snap_Cue.Snap_Cue" 1.0 1.0 0.0 0 0)))))))

(event EventBeginPlay)

(event Collision|EventActorBeginOverlap
  (params (OtherActor :type Actor%20Object%20Reference)))

(event EventTick
  (params (DeltaSeconds :type Float%20%28single-precision%29))
  (if (and (< (Variables|Default|GetTimeSinceTrigger) (Variables|Default|GetSnapDuration)) (Variables|Default|GetboolTriggered))
    (bind _output_get (Variables|Default|SetTimeSinceTrigger (+ DeltaSeconds (Variables|Default|GetTimeSinceTrigger))))
    (Transformation|SetRelativeRotation (Variables|Default|GetClamp) (Math|Rotator|Lerp(Rotator) "0, 0, 0" "0, 0,170.000000" (/ _output_get (Variables|Default|GetSnapDuration)) true) false false)))

(fn ConstructionScript)