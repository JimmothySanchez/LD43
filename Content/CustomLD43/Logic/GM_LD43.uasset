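; Game mode for LD43 that handles Liam's respawning, the cheese-collection goal and map progression.
; On pawn death reported by PC_Liam, it spawns and possesses a new BP_Liam_Parts at the first PlayerStart and counts the death.
; The CameraActor tagged "Active" serves as view target, with its SC_LookAt retargeted to each new pawn.
; It counts BP_Cheese actors at start; when none remain, a delayed timer opens the next map by current level name.
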(event Custom|OnPawnDeath
  ;[1 1 1] Bind event to pawn death
  (CallFunction|SpawnLiam))

(event EventBeginPlay
  (Utilities|FlowControl|Sequence
    (:then_0
      ;[1 1 1] Bind event to pawn death
      (bind _aspc_liam (Utilities|Casting|CastToPC_Liam (Game|GetPlayerController 0)))
      (EventDispatchers|BindEventtoPawnDeath _aspc_liam (delegate Custom|OnPawnDeath)))
    (:then_1
      ;[1 1 1] Set Camera
      (Game|Player|SetViewTargetwithBlend (Game|GetPlayerController 0) (CallFunction|ActiveCamera) 0.0 "VTBlend_Linear" 0.0 false))
    (:then_2
      (CallFunction|InitCheeseCount))
    (:then_3
      ;[1 1 1] FixCamera
      (Variables|/Game/CustomLD43/Actors/Components/SC_LookAt.SC_LookAt_C|SetTarget (Actor|GetComponentbyClass (CallFunction|ActiveCamera) "/Game/CustomLD43/Actors/Components/SC_LookAt.SC_LookAt_C") (Game|Player|GetPlayerPawn 0)))))

(event EventTick
  (params (DeltaSeconds :type Float%20%28single-precision%29)))

(fn ConstructionScript)

(fn SpawnLiam
  (Utilities|FlowControl|Sequence
    (:then_0
      ;[1 1 1] Spawn
      (bind _outactors (Actor|GetAllActorsOfClass "/Script/Engine.PlayerStart"))
      (bind _returnvalue (Game|SpawnActorfromClass "/Game/CustomLD43/Actors/Character/BP_Liam_Parts.BP_Liam_Parts_C" (Transformation|GetActorTransform (Utilities|Array|Get(acopy) _outactors)) "Undefined" 0 (Variables|Default|GetSpawnNudes) 0))
      (LocalVariables|SetlclNewLiam _returnvalue))
    (:then_1
      ;[1 1 1] Posses
      (Pawn|UnPossess (Game|GetPlayerController 0))
      (Pawn|Possess (Game|GetPlayerController 0) (LocalVariables|GetlclNewLiam)))
    (:then_2
      ;[1 1 1] FixCamera
      (Variables|/Game/CustomLD43/Actors/Components/SC_LookAt.SC_LookAt_C|SetTarget (Actor|GetComponentbyClass (CallFunction|ActiveCamera) "/Game/CustomLD43/Actors/Components/SC_LookAt.SC_LookAt_C") (LocalVariables|GetlclNewLiam)))
    (:then_3
      (Math|Integer|IncrementInt (Variables|Default|GetPawnDeathCounter)))))

(fn ActiveCamera
  (bind _outactors (Actor|GetAllActorsOfClass "/Script/Engine.CameraActor"))
  (bind _array_element (Utilities|Array|ForEachLoopwithBreak _outactors)
    (:LoopBody
      (if (Actor|ActorHasTag _array_element "Active")
        (return _array_element)))))

(fn InitCheeseCount
  (bind _outactors (Actor|GetAllActorsOfClass "/Game/CustomLD43/Actors/Traps/BP_Cheese.BP_Cheese_C"))
  (Variables|Default|SetRemainingCheeseCount (Utilities|Array|Length _outactors))
  (for _array_element _outactors
    (EventDispatchers|BindEventtoTriggered _array_element (EventDispatchers|CreateEvent :!event CheeseAquired))))

(fn CheeseAquired
  (bind _result (Math|Integer|DecrementInt (Variables|Default|GetRemainingCheeseCount))
    (:%20%20
      (if (<= _result 0)
        (Utilities|Time|SetTimerbyFunctionName self "LoadNextMap" 3.0)))))

(fn LoadNextMap
  (bind _returnvalue (Game|GetCurrentLevelName true))
  (switch string _returnvalue
    (:Default
      (Game|OpenLevel(byName) "Map1"))
    (:Map1
      (Game|OpenLevel(byName) "Map2"))
    (:Map2
      (Game|OpenLevel(byName) "Map3"))
    (:Map3
      (Game|OpenLevel(byName) "Map_Final"))))